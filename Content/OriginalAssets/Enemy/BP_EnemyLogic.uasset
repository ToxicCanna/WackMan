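; Enemy character Blueprint for WackMan that handles level-based movement speed and resetting to a start position.
; On BeginPlay it stores its location in InitPos, then reads GameLevel from the WackMan game instance to raise walk speed above BaseMoveSpeed, clamped to a cap.
; The CallReset event runs ResetEnemy, which moves the enemy back to InitPos without sweeping.
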(event `CallReset`
  (`self.ResetEnemy`))

(event `self.ReceiveBeginPlay`
  (bind _basemovespeed (`self.BaseMoveSpeed`))
  ;[1 1 1] Init position didnt really work too well, causing bugs on reset, i made these instanced and hardcoded to fix it
  (set `self.InitPos` (`self.K2_GetActorLocation`))
  ;[1 1 1] Set Enemy Walk speed from level variable, maxing at level 20 at 500cm/s
  (bind _aswack_man_game_instance (cast `/Game/OriginalAssets/WackManGameInstance` (`GameplayStatics.GetGameInstance`)))
  (set `CharacterMovementComponent.MaxWalkSpeed` (`KismetMathLibrary.Conv_IntToDouble` (`KismetMathLibrary.Clamp` (+ (* (`/Game/OriginalAssets/WackManGameInstance.GameLevel` _aswack_man_game_instance) 5) _basemovespeed) _basemovespeed 500)) (`self.CharacterMovement`)))

(fn `ResetEnemy`
  (`self.K2_SetActorLocation` (`self.InitPos`)))

(fn `UserConstructionScript`)