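; BP_EnemyRandom is a ghost enemy that wanders randomly and chases the player character on sight.
; On BeginPlay it caches its AIC_RandomWander controller and writes its Range to the blackboard.
; PawnSensing sightings call ChaseTarget on that controller, while capsule overlap with the player calls GhostHit on the game mode.
; The construction script slaves extra skeletal mesh parts to the main Mesh through leader pose.
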(event `self.Capsule.OnComponentBeginOverlap`
  (params (OverlappedComponent :type "PrimitiveComponent Object Reference") (OtherActor :type "Actor Object Reference") (OtherComp :type "PrimitiveComponent Object Reference") (OtherBodyIndex :type Integer) (bFromSweep :type Boolean) (SweepResult :type "HitResult Structure (by ref)"))
  ;[1 1 1] Caught player, call ghosthit
  (cast `/Game/OriginalAssets/BP_ThirdPersonCharacter` OtherActor)
  (bind _asbp_third_person_game_mode (cast `/Game/OriginalAssets/BP_ThirdPersonGameMode` (`GameplayStatics.GetGameMode`)))
  (`/Game/OriginalAssets/BP_ThirdPersonGameMode.GhostHit` _asbp_third_person_game_mode))

(event `self.PawnSensing.OnSeePawn`
  (params (Pawn :type "Pawn Object Reference"))
  ;[1 1 1] Player seen, run em down
  (bind _asbp_third_person_character (cast `/Game/OriginalAssets/BP_ThirdPersonCharacter` Pawn))
  (`/Game/OriginalAssets/Enemy/AIAssets/AIC_RandomWander.ChaseTarget` (`self.RandomController`) _asbp_third_person_character))

(event `self.ReceiveBeginPlay`
  ;[1 1 1] Cache AIC for this enemy
  (bind _asaic_random_wander (cast `/Game/OriginalAssets/Enemy/AIAssets/AIC_RandomWander` (`self.GetController`)))
  (set `self.RandomController` _asaic_random_wander)
  ;[1 1 1] Find Random places to go and set it as target
  (`BlackboardComponent.SetValueAsFloat` (`AIBlueprintHelperLibrary.GetBlackboard` null) "Range" (`self.Range`)))

(fn `UserConstructionScript`
  (`parent.UserConstructionScript`)
  (`SkinnedMeshComponent.SetLeaderPoseComponent` (`self.SkeletalMesh7`) (`self.Mesh`) false false)
  (`SkinnedMeshComponent.SetLeaderPoseComponent` (`self.SkeletalMesh2`) (`self.Mesh`) false false)
  (`SkinnedMeshComponent.SetLeaderPoseComponent` (`self.SkeletalMesh3`) (`self.Mesh`) false false)
  (`SkinnedMeshComponent.SetLeaderPoseComponent` (`self.SkeletalMesh4`) (`self.Mesh`) false false)
  (`SkinnedMeshComponent.SetLeaderPoseComponent` (`self.SkeletalMesh5`) (`self.Mesh`) false false)
  (`SkinnedMeshComponent.SetLeaderPoseComponent` (`self.SkeletalMesh6`) (`self.Mesh`) false false)
  (`SkinnedMeshComponent.SetLeaderPoseComponent` (`self.SkeletalMesh7`) (`self.Mesh`) false false)
  (`SkinnedMeshComponent.SetLeaderPoseComponent` (`self.SkeletalMesh`) (`self.Mesh`) false false)
  (`SkinnedMeshComponent.SetLeaderPoseComponent` (`self.SkeletalMesh1`) (`self.Mesh`) false false)
  (`SkinnedMeshComponent.SetLeaderPoseComponent` (`self.SkeletalMesh8`) (`self.Mesh`) false false))