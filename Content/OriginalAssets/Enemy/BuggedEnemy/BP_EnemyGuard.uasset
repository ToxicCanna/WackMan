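; BP_EnemyGuard is an enemy guard that patrols, senses the player and triggers GhostHit on the game mode when its capsule overlaps the player.
; PawnSensing passes seen players to the AIC_Guard controller to chase and heard noise locations to investigate.
; PatrolRoute advances the patrol point index, either looping or reversing at the path's end.
; Construction links modular skeletal meshes to the main mesh as leader pose.
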(event `self.ReceiveBeginPlay`
  (bind _asaic_guard (cast `/Game/OriginalAssets/Enemy/BuggedEnemy/AIC_Guard` (`self.GetController`)))
  (set `self.GuardController` _asaic_guard))

(event `self.Capsule.OnComponentBeginOverlap`
  (params (OverlappedComponent :type "PrimitiveComponent Object Reference") (OtherActor :type "Actor Object Reference") (OtherComp :type "PrimitiveComponent Object Reference") (OtherBodyIndex :type Integer) (bFromSweep :type Boolean) (SweepResult :type "HitResult Structure (by ref)"))
  (cast `/Game/OriginalAssets/BP_ThirdPersonCharacter` OtherActor)
  (bind _asbp_third_person_game_mode (cast `/Game/OriginalAssets/BP_ThirdPersonGameMode` (`GameplayStatics.GetGameMode`)))
  (`/Game/OriginalAssets/BP_ThirdPersonGameMode.GhostHit` _asbp_third_person_game_mode))

(event `self.PawnSensing.OnSeePawn`
  (params (Pawn :type "Pawn Object Reference"))
  (bind _asbp_third_person_character (cast `/Game/OriginalAssets/BP_ThirdPersonCharacter` Pawn))
  (`/Game/OriginalAssets/Enemy/BuggedEnemy/AIC_Guard.ChaseTarget` (`self.GuardController`) _asbp_third_person_character))

(event `self.PawnSensing.OnHearNoise`
  (params (Instigator :type "Pawn Object Reference") (Location :type "Vector Structure (by ref)") (Volume :type "Float (single-precision)"))
  (`/Game/OriginalAssets/Enemy/BuggedEnemy/AIC_Guard.Investigate` (`self.GuardController`) Location))

(fn `PatrolRoute`
  (if (`self.bForward`)
    (bind _result (`/Engine/EditorBlueprintResources/StandardMacros.IncrementInt` (`self.CurrentPatrolPoint`))
      (:`  `
        (if (`/Game/OriginalAssets/Enemy/AIAssets/BP_Path.AtEndOfPath` (`self.PatrolPath`) _result)
          (if (`/Game/OriginalAssets/Enemy/AIAssets/BP_Path.bLooping` (`self.PatrolPath`))
            (set `self.CurrentPatrolPoint` 0)
            (else
              (set `self.bForward` false))))))
    (else
      (bind _result_2 (`/Engine/EditorBlueprintResources/StandardMacros.DecrementInt` (`self.CurrentPatrolPoint`))
        (:`  `
          (if (<= _result_2 0)
            (set `self.bForward` true)))))))

(fn `UserConstructionScript`
  (`SkinnedMeshComponent.SetLeaderPoseComponent` (`self.SkeletalMesh7`) (`self.Mesh`) false false)
  (`SkinnedMeshComponent.SetLeaderPoseComponent` (`self.SkeletalMesh2`) (`self.Mesh`) false false)
  (`SkinnedMeshComponent.SetLeaderPoseComponent` (`self.SkeletalMesh3`) (`self.Mesh`) false false)
  (`SkinnedMeshComponent.SetLeaderPoseComponent` (`self.SkeletalMesh4`) (`self.Mesh`) false false)
  (`SkinnedMeshComponent.SetLeaderPoseComponent` (`self.SkeletalMesh5`) (`self.Mesh`) false false)
  (`SkinnedMeshComponent.SetLeaderPoseComponent` (`self.SkeletalMesh6`) (`self.Mesh`) false false)
  (`SkinnedMeshComponent.SetLeaderPoseComponent` (`self.SkeletalMesh7`) (`self.Mesh`) false false)
  (`SkinnedMeshComponent.SetLeaderPoseComponent` (`self.SkeletalMesh`) (`self.Mesh`) false false)
  (`SkinnedMeshComponent.SetLeaderPoseComponent` (`self.SkeletalMesh1`) (`self.Mesh`) false false)
  (`SkinnedMeshComponent.SetLeaderPoseComponent` (`self.SkeletalMesh8`) (`self.Mesh`) false false))